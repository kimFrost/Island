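; Line actor that draws a mesh segment between the From and To points, with an Arrow at the end.
; The construction script rebuilds a two-point spline, reading From in local space and To in local or world space depending on LocalTo.
; The spline's endpoint positions and tangents shape the spline mesh, and its end point places and orients the Arrow.
; All logic runs at construction, and the event graph is empty.
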(event `self.ReceiveBeginPlay`)

(event `self.ReceiveActorBeginOverlap`
  (params (OtherActor :type "Actor Object Reference")))

(event `self.ReceiveTick`
  (params (DeltaSeconds :type "Float (single-precision)")))

(fn `UserConstructionScript`
  (bind _spline (`self.Spline`))
  (bind _spline_2 (`self.Spline`))
  (bind (_location _tangent) (`SplineComponent.GetLocationAndTangentAtSplinePoint` _spline 1 "Local"))
  (bind (_location_2 _tangent_2) (`SplineComponent.GetLocationAndTangentAtSplinePoint` _spline 0 "Local"))
  (`|ExecutionSequence`
    (:`then_0`
      (`SplineComponent.ClearSplinePoints` _spline_2)
      (`SplineComponent.AddSplinePoint` _spline_2 (`self.From`) "Local")
      (`SplineComponent.AddSplinePoint` _spline_2 (`self.To`) (select `bool` (`self.LocalTo`) :`false` "World" :`true` "Local" :!type "ESplineCoordinateSpace Enum")))
    (:`then_1`
      (`|ExecutionSequence`
        (:`then_0`
          (`SplineMeshComponent.SetStartAndEnd` (`self.SplineMesh`) _location_2 _tangent_2 _location _tangent))
        (:`then_1`
          (`SceneComponent.K2_SetRelativeLocationAndRotation` (`self.Arrow`) _location (`SplineComponent.GetRotationAtSplinePoint` _spline 1 "Local") false false))))))