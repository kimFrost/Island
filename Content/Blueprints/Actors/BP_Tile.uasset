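; BP_Tile is a tile actor that links to other tiles or actors through its PathTo array and shows those connections visually.
; The construction script draws short-lived green debug lines to each linked actor as a preview of the connections.
; On BeginPlay it spawns one BP_Line per link at its own location, passing the target as a local offset.
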(event `self.ReceiveBeginPlay`
  (bind _returnvalue (`self.K2_GetActorLocation`))
  (for _array_element (`self.PathTo`)
    (`|SpawnActorFromClass` "/Game/Blueprints/Actors/BP_Line.BP_Line_C" (`KismetMathLibrary.MakeTransform` _returnvalue) "Undefined" "OverrideRootScale" null (0.0 0.0 0.0) (- (`self.K2_GetActorLocation` _array_element) _returnvalue) true)))

(event `self.ReceiveActorBeginOverlap`
  (params (OtherActor :type "Actor Object Reference")))

(event `self.ReceiveTick`
  (params (DeltaSeconds :type "Float (single-precision)")))

(fn `UserConstructionScript`
  (for _array_element (`self.PathTo`)
    (`KismetSystemLibrary.DrawDebugLine` (`self.K2_GetActorLocation`) (`self.K2_GetActorLocation` _array_element) (struct :`G` 1.0 :`B` 0.118933 :`A` 1.0) 2.0 20.0)))